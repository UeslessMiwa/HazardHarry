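; Blueprint function library with shared helpers for the Harry player character and interactable item setup.
; EditorAddItem maps a weapon selection, fixed or random, to a row name and returns that row from the DT_ItemIndex data table; only the Weapon item type is handled.
; CastToHarry returns the first player's pawn as BP_Harry.
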(fn `Cast to Harry`
  (returns (`Harry Ref` :type "/Game/FirstPerson/Blueprints/BP_Harry Object Reference"))
  (bind _asbp_harry (cast `/Game/FirstPerson/Blueprints/BP_Harry` (`GameplayStatics.GetPlayerPawn` null)))
  (return _asbp_harry))

(fn `Editor Add Item`
  (params (`Item Type` :type "/Game/Blueprints/Interactables/Pickups/EN_ItemType Enum" :default "NewEnumerator0") (`Selection (Weapon)` :type "/Game/Blueprints/Interactables/Pickups/EN_WeaponList Enum" :default "NewEnumerator0"))
  (returns (`ST Item Data` :type "/Game/Blueprints/Interactables/Pickups/ST_ItemData Structure"))
  (locals (`ST Item Data` :type "/Game/Blueprints/Interactables/Pickups/ST_ItemData Structure") (`Row Num` :type Integer :default 5) (`Row Names (Weapons)` :type "Array of Name"))
  (switch `/Game/Blueprints/Interactables/Pickups/EN_ItemType` `Item Type`
    (:`NewEnumerator0`
      (switch `/Game/Blueprints/Interactables/Pickups/EN_WeaponList` `Selection (Weapon)`
        (:`NewEnumerator0`
          (set `local.Row Num` 0))
        (:`NewEnumerator1`
          (set `local.Row Num` 1))
        (:`NewEnumerator2`
          (set `local.Row Num` 2))
        (:`NewEnumerator3`
          (set `local.Row Num` 3))
        (:`NewEnumerator4`
          (set `local.Row Num` 4))
        (:`NewEnumerator5`
          (set `local.Row Num` 5))
        (:`NewEnumerator6`
          (set `local.Row Num` (`KismetMathLibrary.RandomIntegerInRange` 0 (`local.Row Num`)))))
      (bind _returnvalue (`|GetDataTableRow` "/Game/Blueprints/Interactables/Pickups/DT_ItemIndex.DT_ItemIndex" (`|GetArrayItem` (`local.Row Names (Weapons)`) (`local.Row Num`)))
        (:`then`
          (return _returnvalue))))))