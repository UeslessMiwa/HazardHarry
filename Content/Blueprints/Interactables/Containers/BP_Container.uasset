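; Lootable container that the player opens in the inventory HUD, with mesh, name and size taken from a DT_ContainerIndex row in the construction script.
; On BeginPlay it creates its slots and fills them by rolling each DT_ItemIndex item's SpawnRate once per pass over the container size.
; Closing packs filled slots into StoredData with an empty-slot count, and opening rebuilds the inventory from both.
; AddItem places items in the first free slot.
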(event `Random Weighted Fill`)

(event `Editor Add Item`
  ;[1 1 1 0.5 40] Editor add item
  (bind _st_item_data (`/Game/Blueprints/Interactables/BPF_HarryBP.Editor Add Item` (`self.Item Type`) (`self.Selection (Weapon)`)))
  (`self.Add Item` _st_item_data))

(event `Random Fill`
  (for _index (range (+ (`self.Container Space`) 1))
    (bind _st_item_data (`/Game/Blueprints/Interactables/BPF_HarryBP.Editor Add Item` "NewEnumerator0" "NewEnumerator6"))
    (bind _returnvalue (`|GetDataTableRow` "/Game/Blueprints/Interactables/Pickups/DT_ItemIndex.DT_ItemIndex" (`.Name_39_DCB06C934239801CA588FCBD1C74C308` (break `/Game/Blueprints/Interactables/Pickups/ST_ItemData` _st_item_data)))
      (:`then`
        (`KismetArrayLibrary.Array_Set` (`self.Container Inventory`) _index _returnvalue)))))

(event `self.ReceiveBeginPlay`
  (bind (_st_container_data_locked_ _st_container_data_actorref _st_container_data_actorclass _st_container_data_containermesh _st_container_data_containername _st_container_data_containersize) (break `/Game/Blueprints/Interactables/Containers/ST_ContainerData` (`self.ST Container Data`)))
  ;[1 1 1 0.5 40] Cast to harry
  (bind _harry_ref (`/Game/Blueprints/Interactables/BPF_HarryBP.Cast to Harry`))
  (set `self.Harry Ref` _harry_ref)
  (for _ (range 1 (+ _st_container_data_containersize 1))
    (`KismetArrayLibrary.Array_Add` (`self.Container Inventory`)))
  (`self.Random Items (Weighted)`))

(event `EnhancedInput|/Game/Input/Actions/IA_Inventory`
  (params (ActionValue :type Boolean) (ElapsedSeconds :type "Float (double-precision)") (TriggeredSeconds :type "Float (double-precision)") (InputAction :type "InputAction Object Reference" :default "/Game/Input/Actions/IA_Inventory.IA_Inventory"))
  ;[0.15 0.07415 0.06985 0.5 40] Close menu
  (:`Started`
    (`self.Store Container Data`)
    (`/Game/FirstPerson/Blueprints/BP_Harry.Set Inventory HUD` (`self.Harry Ref`) false "NewEnumerator0" true)))

(event `Store Container Data`
  ;[0.04246 0.04271 0.15 0.5 40] Close widget and store the container data
  (`|ExecutionSequence`
    (:`then_0`
      ;; Store data in different array
      (set `self.Extra space` -1)
      (`KismetArrayLibrary.Array_Clear` (`self.Stored Data`))
      (for _array_element (`self.Container Inventory`)
        (if (`KismetSystemLibrary.IsValidClass` (`.ActorClass_35_6CAA728E446A3208DD0AAAA301EAD167` (break `/Game/Blueprints/Interactables/Pickups/ST_ItemData` _array_element)))
          (`KismetArrayLibrary.Array_Add` (`self.Stored Data`) _array_element)
          (else
            (`/Engine/EditorBlueprintResources/StandardMacros.IncrementInt` (`self.Extra space`))))))
    (:`then_1`
      ;; Clear inventory leftover data
      (`KismetArrayLibrary.Array_Clear` (`self.Container Inventory`))
      (`self.DisableInput` (`GameplayStatics.GetPlayerController` 0)))))

(event `Open Container`
  ;[0.05838 0.0789 0.15 0.5 40] Open Container rules
  (`|ExecutionSequence`
    (:`then_0`
      (if (`KismetArrayLibrary.Array_IsEmpty` (`self.Stored Data`))
        ;;[0.15 0.1183 0.08051 0.5] If container is completely empty when player tries to add item then create new slot.
        (if (`KismetArrayLibrary.Array_IsEmpty` (`self.Container Inventory`))
          (for _ (range (+ (`self.Container Space`) 1))
            (`KismetArrayLibrary.Array_Add` (`self.Container Inventory`))
            (`/Game/FirstPerson/Blueprints/BP_Harry.Set Inventory HUD` (`self.Harry Ref`) true "NewEnumerator1" true :!label _label)
            (`self.EnableInput` (`GameplayStatics.GetPlayerController` 0)))
          (else
            (goto _label)))
        (else
          ;;[0.15 0.1344 0.09165 0.5] Add stored data back to container inventory
          (for _array_element (`self.Stored Data`)
            (`KismetArrayLibrary.Array_Add` (`self.Container Inventory`) _array_element))
          (for _ (range (+ (`self.Extra space`) 1))
            (`KismetArrayLibrary.Array_Add` (`self.Container Inventory`)))
          (`/Game/FirstPerson/Blueprints/BP_Harry.Set Inventory HUD` (`self.Harry Ref`) true "NewEnumerator1" true)
          (`self.EnableInput` (`GameplayStatics.GetPlayerController` 0)))))
    (:`then_1`
      ;;[0.15 0.1322 0.07469 0.5] Reset and then set the container limit text
      (set `self.Filled Space` 0)
      (for _array_element_2 (`self.Container Inventory`)
        (if (`KismetSystemLibrary.IsValidClass` (`.ActorClass_35_6CAA728E446A3208DD0AAAA301EAD167` (break `/Game/Blueprints/Interactables/Pickups/ST_ItemData` _array_element_2)))
          (`/Engine/EditorBlueprintResources/StandardMacros.IncrementInt` (`self.Filled Space`)))))))

(fn `Add Item`
  (params (`Item Data Ref` :type "/Game/Blueprints/Interactables/Pickups/ST_ItemData Structure") (Debug :type Boolean))
  (returns (`Found Slot?` :type Boolean) (`Item Slot Num` :type Integer))
  (set `self.Item Data Ref` `Item Data Ref`)
  (for (_array_element _array_index) (`self.Container Inventory`)
    (bind _returnvalue (`KismetSystemLibrary.IsValidClass` (`.ActorClass_35_6CAA728E446A3208DD0AAAA301EAD167` (break `/Game/Blueprints/Interactables/Pickups/ST_ItemData` _array_element))))
    (if _returnvalue
      (if (and (== (`KismetArrayLibrary.Array_LastIndex` (`self.Container Inventory`)) _array_index) _returnvalue)
        (`|ExecutionSequence`
          (:`then_0`
            (break))
          (:`then_1`
            (bind _output_get (set `self.Found Slot` false))
            (return _output_get (stale _output_get_2)))))
      (else
        (set `self.Found Slot` true)
        (bind _output_get_2 (set `self.Slot Num` _array_index))
        (`KismetSystemLibrary.PrintString` "Inventory Space Found." Debug)
        (`|ExecutionSequence`
          (:`then_0`
            (`KismetArrayLibrary.Array_Set` (`self.Container Inventory`) (`self.Slot Num`) (`self.Item Data Ref`)))
          (:`then_1`
            (`KismetSystemLibrary.PrintString` (`KismetStringLibrary.Conv_NameToString` (`.Name_39_DCB06C934239801CA588FCBD1C74C308` (break `/Game/Blueprints/Interactables/Pickups/ST_ItemData` (`self.Item Data Ref`)))) Debug))
          (:`then_2`
            (break))
          (:`then_3`
            (return (`self.Found Slot`) (`self.Slot Num`))))))))

(fn `Random Items (Weighted)`
  (locals (`Item List` :type "Array of Name") (`All Items` :type "Array of /Game/Blueprints/Interactables/Pickups/ST_ItemData Structure") (`Items to Spawn` :type "Array of /Game/Blueprints/Interactables/Pickups/ST_ItemData Structure"))
  (bind (_st_container_data_locked_ _st_container_data_actorref _st_container_data_actorclass _st_container_data_containermesh _st_container_data_containername _st_container_data_containersize) (break `/Game/Blueprints/Interactables/Containers/ST_ContainerData` (`self.ST Container Data`)))
  (bind _outrownames (`DataTableFunctionLibrary.GetDataTableRowNames` "/Game/Blueprints/Interactables/Pickups/DT_ItemIndex.DT_ItemIndex"))
  (for _array_element _outrownames
    (`KismetArrayLibrary.Array_Add` (`local.Item List`) _array_element))
  (for _array_element_2 (`local.Item List`)
    (bind _returnvalue (`|GetDataTableRow` "/Game/Blueprints/Interactables/Pickups/DT_ItemIndex.DT_ItemIndex" _array_element_2)
      (:`then`
        (`KismetArrayLibrary.Array_Add` (`local.All Items`) _returnvalue))))
  (for _ (range (+ _st_container_data_containersize 1))
    (for _array_element_3 (`local.All Items`)
      (bind (_actorclass _actormesh _actorref _spawned_ _icon _name _description _type _material _damage _class _armor _weight _value _itemcount _spawnrate) (break `/Game/Blueprints/Interactables/Pickups/ST_ItemData` _array_element_3))
      (if (<= (`KismetMathLibrary.RandomFloatInRange` 0.0 100.0) _spawnrate)
        (`KismetSystemLibrary.PrintString` (`KismetStringLibrary.Conv_NameToString` _name) true true (struct :`G` 1.0 :`B` 0.031242 :`A` 0.5))
        (`KismetArrayLibrary.Array_Add` (`local.Items to Spawn`) _array_element_3))))
  (for (_array_element_4 _array_index) (`local.Items to Spawn`)
    (`KismetArrayLibrary.Array_Set` (`self.Container Inventory`) _array_index _array_element_4)))

(fn `UserConstructionScript`
  (locals (NewLocalVar :type Integer :default 0))
  (bind _container_type (`self.Container Type`))
  ;[0.02374 0.04283 0.15 0.5 40] Setup for container mesh
  (bind _outrownames (`DataTableFunctionLibrary.GetDataTableRowNames` "/Game/Blueprints/Interactables/Containers/DT_ContainerIndex.DT_ContainerIndex"))
  (for (_array_element _array_index) _outrownames
    (`KismetArrayLibrary.Array_AddUnique` _container_type _array_element)
    (`KismetArrayLibrary.Array_Set` _container_type _array_index _array_element))
  (bind _returnvalue (`|GetDataTableRow` "/Game/Blueprints/Interactables/Containers/DT_ContainerIndex.DT_ContainerIndex" (`|GetArrayItem` (`self.Container Type`) (`self.Container Type Num`)))
    (:`then`
      ;; Individual container item data
      (set `self.ST Container Data` (make `/Game/Blueprints/Interactables/Containers/ST_ContainerData` (break `/Game/Blueprints/Interactables/Containers/ST_ContainerData` _returnvalue) (`.ActorRef_27_4F9C31DF42699044EB2DA0A220029D3C` (break `/Game/Blueprints/Interactables/Containers/ST_ContainerData` _returnvalue)) (`.ActorClass_26_DF0F06C249C09610F5C09298F053EB7F` (break `/Game/Blueprints/Interactables/Containers/ST_ContainerData` _returnvalue)) (`.ContainerMesh_24_9091226D4158701B4C3CBF85CB41D198` (break `/Game/Blueprints/Interactables/Containers/ST_ContainerData` _returnvalue)) (`.ContainerName_23_6D3857274CD7ED1D9702A280F0645BB5` (break `/Game/Blueprints/Interactables/Containers/ST_ContainerData` _returnvalue)) (`.ContainerSize_43_325380FC4741F7C59121ACA1C04CFDE0` (break `/Game/Blueprints/Interactables/Containers/ST_ContainerData` _returnvalue))))
      (`StaticMeshComponent.SetStaticMesh` (`self.StaticMesh`) (`.ContainerMesh_24_9091226D4158701B4C3CBF85CB41D198` (break `/Game/Blueprints/Interactables/Containers/ST_ContainerData` _returnvalue))))))