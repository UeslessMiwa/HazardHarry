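; World pickup item whose data and mesh come from the DT_ItemIndex data table.
; The construction script fills the item struct and mesh from the row at RowNum, and BeginPlay re-rolls a random row when Randomize is set.
; InteractRadius toggles input as BP_Harry enters or leaves.
; Pickup hides the actor rather than destroying it, and dropping moves it to Harry's look-at point, restoring physics after a short delay.
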(event `self.Interact Radius.OnComponentBeginOverlap`
  (params (OverlappedComponent :type "PrimitiveComponent Object Reference") (OtherActor :type "Actor Object Reference") (OtherComp :type "PrimitiveComponent Object Reference") (OtherBodyIndex :type Integer) (bFromSweep :type Boolean) (SweepResult :type "HitResult Structure (by ref)"))
  ;[0.15 0.15 0.15 0.5 40] Item input
  (if (== (`GameplayStatics.GetObjectClass` OtherActor) "/Game/FirstPerson/Blueprints/BP_Harry.BP_Harry_C")
    (bind _asbp_harry (cast `/Game/FirstPerson/Blueprints/BP_Harry` OtherActor))
    (set `self.Harry Ref` _asbp_harry)
    (`KismetSystemLibrary.PrintString` "Enter Item Radius" (`self.Print Debug?`))
    (`self.EnableInput` (`GameplayStatics.GetPlayerController` 0))))

(event `self.Interact Radius.OnComponentEndOverlap`
  (params (OverlappedComponent :type "PrimitiveComponent Object Reference") (OtherActor :type "Actor Object Reference") (OtherComp :type "PrimitiveComponent Object Reference") (OtherBodyIndex :type Integer))
  ;[0.15 0.15 0.15 0.5 40] Item input
  (if (== (`GameplayStatics.GetObjectClass` OtherActor) "/Game/FirstPerson/Blueprints/BP_Harry.BP_Harry_C")
    (`self.DisableInput` (`GameplayStatics.GetPlayerController` 0) null)))

(event `Item Picked Up`
  (params (`Space Found?` :type Boolean :default true))
  ;[0.15 0.15 0.15 0.5 40] Pick up item
  (if `Space Found?`
    (`self.SetActorEnableCollision` false)
    (`self.SetActorHiddenInGame` true)
    (`PrimitiveComponent.SetSimulatePhysics` (`self.StaticMesh`) false)
    (`KismetSystemLibrary.PrintString` "Item picked up." (`self.Print Debug?`))))

(event `Item Dropped`
  (bind _harry_ref (`self.Harry Ref`))
  ;[0.15 0.15 0.15 0.5 40] Drop item
  (bind _look_at_location (`/Game/FirstPerson/Blueprints/BP_Harry.Get Look At` _harry_ref))
  (`self.K2_SetActorLocationAndRotation` _look_at_location (`self.K2_GetActorRotation` _harry_ref))
  (`self.SetActorHiddenInGame` false)
  (`KismetSystemLibrary.Delay` 0.1)
  (`PrimitiveComponent.SetSimulatePhysics` (`self.StaticMesh`) true)
  (`self.SetActorEnableCollision` true))

(event `self.ReceiveBeginPlay`
  ;[0.15 0.15 0.15 0.5 40] Comment
  (if (`self.Randomize`)
    (bind _returnvalue (`|GetDataTableRow` "/Game/Blueprints/Interactables/Pickups/DT_ItemIndex.DT_ItemIndex" (`KismetArrayLibrary.Array_Random` (`self.Row Name`)))
      (:`then`
        (bind (_actorclass _actormesh _actorref _spawned_ _icon _name _description _type _material _damage _class _armor _weight _value _itemcount) (break `/Game/Blueprints/Interactables/Pickups/ST_ItemData` _returnvalue))
        (set `self.ST Item Data` (make `/Game/Blueprints/Interactables/Pickups/ST_ItemData` _actorclass _actormesh self _spawned_ _icon _name _description _type _material _damage _class _armor _weight _value _itemcount))
        (`StaticMeshComponent.SetStaticMesh` (`self.StaticMesh`) _actormesh)
        (`self.SetActorEnableCollision` false)
        (`PrimitiveComponent.SetSimulatePhysics` (`self.StaticMesh`) false)
        (`KismetSystemLibrary.Delay` 0.1)
        (`PrimitiveComponent.SetSimulatePhysics` (`self.StaticMesh`) true)
        (`self.SetActorEnableCollision` true)))))

(fn `UserConstructionScript`
  (bind _row_name (`self.Row Name`))
  (bind _outrownames (`DataTableFunctionLibrary.GetDataTableRowNames` "/Game/Blueprints/Interactables/Pickups/DT_ItemIndex.DT_ItemIndex"))
  (for (_array_element _array_index) _outrownames
    (`KismetArrayLibrary.Array_AddUnique` _row_name _array_element)
    (`KismetArrayLibrary.Array_Set` _row_name _array_index _array_element))
  (bind _returnvalue (`|GetDataTableRow` "/Game/Blueprints/Interactables/Pickups/DT_ItemIndex.DT_ItemIndex" (`|GetArrayItem` (`self.Row Name`) (`self.Row Num`)))
    (:`then`
      (bind (_actorclass _actormesh _actorref _spawned_ _icon _name _description _type _material _damage _class _armor _weight _value _itemcount) (break `/Game/Blueprints/Interactables/Pickups/ST_ItemData` _returnvalue))
      (set `self.ST Item Data` (make `/Game/Blueprints/Interactables/Pickups/ST_ItemData` _actorclass _actormesh self _spawned_ _icon _name _description _type _material _damage _class _armor _weight _value _itemcount))
      (`StaticMeshComponent.SetStaticMesh` (`self.StaticMesh`) _actormesh))))